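; Level game manager actor that handles tutorial, pause and level completion for a flower-blooming level.
; When three triggers all report full bloom, it shows the completion widget, locks player input and loops a cinematic.
; Escape or gamepad Start opens the pause menu and pauses the tutorial animation, saving its time; gamepad Back reloads Level_1.
; It also counts unlocked secret flowers from seven flags for the UI.
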(event `CheckBloomedFlowers`
  (bind _returnvalue (`GameplayStatics.GetPlayerController` 0))
  (bind _bloomedalla (`/Game/Blueprints/BP_TB_PollenA_Trigger.BloomedAllA` (`self.Trigger A`)))
  (bind _bloomedallb (`/Game/Blueprints/BP_TB_PollenB_Trigger.BloomedAllB` (`self.Trigger B`)))
  (bind _bloomedallc (`/Game/Blueprints/BP_TB_PollenC_Trigger.BloomedAllC` (`self.Trigger C`)))
  (if (and _bloomedalla _bloomedallb _bloomedallc)
    (bind _returnvalue_2 (`|CreateWidget` "/Game/Blueprints/WBP_LevelComplete.WBP_LevelComplete_C" _returnvalue))
    (`UserWidget.AddToViewport` _returnvalue_2 0)
    (`WidgetBlueprintLibrary.SetInputMode_UIOnlyEx` _returnvalue _returnvalue_2)
    (set `PlayerController.bShowMouseCursor` true _returnvalue)
    (`Controller.SetIgnoreLookInput` _returnvalue true)
    (`Controller.SetIgnoreMoveInput` _returnvalue true)
    (`MovieSceneSequencePlayer.PlayLooping` (`LevelSequenceActor.SequencePlayer` (`self.LS_LevelCompleteCine`)) -1)
    (else
      (`KismetSystemLibrary.PrintString` (`KismetStringLibrary.Conv_BoolToString` _bloomedalla))
      (`KismetSystemLibrary.PrintString` (`KismetStringLibrary.Conv_BoolToString` _bloomedallb))
      (`KismetSystemLibrary.PrintString` (`KismetStringLibrary.Conv_BoolToString` _bloomedallc)))))

(event `self.ReceiveBeginPlay`
  (bind _returnvalue (`GameplayStatics.GetPlayerController` 0))
  (set `self.SecretFlowersArray` (`|MakeArray` (`self.SecretFlower1Unlocked`) (`self.SecretFlower2Unlocked`) (`self.SecretFlower3Unlocked`) (`self.SecretFlower4Unlocked`) (`self.SecretFlower5Unlocked`) (`self.SecretFlower6Unlocked`) (`self.SecretFlower7Unlocked`)))
  (`WidgetBlueprintLibrary.SetInputMode_GameOnly` _returnvalue)
  (bind _returnvalue_2 (`|CreateWidget` "/Game/Blueprints/WBP_Tutorial.WBP_Tutorial_C" _returnvalue))
  (`UserWidget.AddToViewport` _returnvalue_2 0))

(event `Key|Gamepad_Special_Right`
  (params (Key :type "Key Structure"))
  (bind _returnvalue (`GameplayStatics.GetPlayerController` 0))
  (:`Pressed`
    (bind _returnvalue_2 (`|CreateWidget` "/Game/Blueprints/WBP_Pause.WBP_Pause_C" _returnvalue :!label _label))
    (`UserWidget.AddToViewport` _returnvalue_2 0)
    (`WidgetBlueprintLibrary.SetInputMode_UIOnlyEx` _returnvalue _returnvalue_2)
    (set `PlayerController.bShowMouseCursor` true _returnvalue)
    (`Controller.SetIgnoreLookInput` _returnvalue false)
    (`Controller.SetIgnoreMoveInput` _returnvalue true)
    (`GameplayStatics.SetGamePaused` true)
    ;[1 1 1] Pause Animation
    (bind _foundwidgets (`WidgetBlueprintLibrary.GetAllWidgetsOfClass` "/Game/Blueprints/WBP_Tutorial.WBP_Tutorial_C" false))
    (bind _output (`|GetArrayItem` _foundwidgets))
    (`/Engine/EditorBlueprintResources/StandardMacros.IsValid` _output
      (:`Is Valid`
        (bind _returnvalue_3 (`UserWidget.PauseAnimation` _output (`/Game/Blueprints/WBP_Tutorial.Tutorial0` _output)))
        (set `self.PausedAnimationCurrentTime` _returnvalue_3))
      (:`Is Not Valid`
        _))
    (set `self.IsPaused` true)))

(event `Key|Escape`
  (params (Key :type "Key Structure"))
  (:`Pressed`
    (goto _label)))

(event `Key|Gamepad_Special_Left`
  (params (Key :type "Key Structure"))
  (:`Pressed`
    (`GameplayStatics.OpenLevel` "Level_1")))

(fn `SecretFlowersCollectedUICheck`
  (bind _secretflowerscollectedui (`self.SecretFlowersCollectedUI`))
  (`self.UpdateSecretFlowerArray`)
  (set `self.SecretFlowersCollectedUI` 0)
  (for _array_element (`self.SecretFlowersArray`)
    (if _array_element
      (bind _result (`/Engine/EditorBlueprintResources/StandardMacros.IncrementInt` _secretflowerscollectedui)
        (:`  `
          (set `self.SecretFlowersCollectedUI` _result)))))
  (`KismetSystemLibrary.PrintString` (`KismetStringLibrary.Conv_IntToString` _secretflowerscollectedui)))

(fn `UpdateSecretFlowerArray`
  (set `self.SecretFlowersArray` (`|MakeArray` (`self.SecretFlower1Unlocked`) (`self.SecretFlower2Unlocked`) (`self.SecretFlower3Unlocked`) (`self.SecretFlower4Unlocked`) (`self.SecretFlower5Unlocked`) (`self.SecretFlower6Unlocked`) (`self.SecretFlower7Unlocked`))))

(fn `UserConstructionScript`)