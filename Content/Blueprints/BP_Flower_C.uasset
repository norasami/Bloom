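; BP_Flower_C is a flower that hands type C pollen to the bee.
; BeginPlay sets its pollen particle to match HasPollen.
; On Box overlap, it casts the stored Bee reference, not the overlapping actor; if that bee carries no pollen and HasPollen is true, the particle and pollen state move to the bee.
; FlowerCPollenOff separately clears the flower's particle and HasPollen.
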(event `self.ReceiveBeginPlay`
  (if (`self.hasPollen`)
    (`ActorComponent.SetActive` (`self.P_FlowerPollenC`) true false)
    (else
      (`ActorComponent.SetActive` (`self.P_FlowerPollenC`) false false))))

(event `self.Box.OnComponentBeginOverlap`
  (params (OverlappedComponent :type "PrimitiveComponent Object Reference") (OtherActor :type "Actor Object Reference") (OtherComp :type "PrimitiveComponent Object Reference") (OtherBodyIndex :type Integer) (bFromSweep :type Boolean) (SweepResult :type "HitResult Structure (by ref)"))
  ;[1 1 1] If the bee has no pollen
  (bind _asbp_bee (cast `/Game/Blueprints/BP_Bee` (`self.Bee`)))
  (if (not (or (`/Game/Blueprints/BP_Bee.pollenACollected` _asbp_bee) (`/Game/Blueprints/BP_Bee.pollenBCollected` _asbp_bee) (`/Game/Blueprints/BP_Bee.pollenCCollected` _asbp_bee)))
    ;[1 1 1] If the flower has pollen and the bee doesn't
    (if (`self.hasPollen`)
      (bind _asbp_bee_2 (cast `/Game/Blueprints/BP_Bee` (`self.Bee`)))
      (if (not (`/Game/Blueprints/BP_Bee.pollenCCollected` _asbp_bee_2))
        ;[1 1 1] Turn pollen off the flower and on, on the bee
        (`ActorComponent.SetActive` (`self.P_FlowerPollenC`) false false)
        (bind _asbp_bee_3 (cast `/Game/Blueprints/BP_Bee` (`self.Bee`)))
        (`ActorComponent.SetActive` (`/Game/Blueprints/BP_Bee.P_BeePollenC` _asbp_bee_3) true false)
        (set `/Game/Blueprints/BP_Bee.pollenCCollected` true _asbp_bee_3)
        (set `self.hasPollen` false)))))

(fn `FlowerCPollenOff`
  (`ActorComponent.SetActive` (`self.P_FlowerPollenC`) false false)
  (set `self.hasPollen` false))

(fn `UserConstructionScript`)