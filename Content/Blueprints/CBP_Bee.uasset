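; Player-controlled bee Character that takes off, flies with boost and reverse, and lands on the landscape.
; Input switches movement mode between None and Flying, with delays matching takeoff and landing animations flagged on ABP_Bee.
; Landscape hits set CanLand, never cleared here, making backward input land instead of reverse.
; Spring arm camera turns with interpolated input and limited pitch; BeginPlay sets three pollen effects from collection flags, and ReturnCamera blends view targets.
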(event `InputAxis|LookUp`
  (params (AxisValue :type "Float (single-precision)"))
  (bind _returnvalue (`GameplayStatics.GetWorldDeltaSeconds`))
  ;[1 1 1] Rotation Input
  (if (`NavMovementComponent.IsFlying` (`self.CharacterMovement`))
    (if (`self.InvertMouseControl`)
      (`self.AddControllerPitchInput` (* (* AxisValue -1.0) (`self.BeeLookUpRate`) _returnvalue))
      (else
        (`self.AddControllerPitchInput` (* AxisValue (`self.BeeTurnRate`) _returnvalue))))))

(event `InputAxis|Turn`
  (params (AxisValue :type "Float (single-precision)"))
  ;[1 1 1] Rotation Input
  (if (`NavMovementComponent.IsFlying` (`self.CharacterMovement`))
    (`self.AddControllerYawInput` (* AxisValue (`self.BeeTurnRate`) (`GameplayStatics.GetWorldDeltaSeconds`)))))

(event `self.ReceiveBeginPlay`
  (bind _charactermovement (`self.CharacterMovement`))
  (`CharacterMovementComponent.SetMovementMode` _charactermovement "MOVE_None" 0)
  (set `CharacterMovementComponent.MaxFlySpeed` (`self.Max Fly Speed`) _charactermovement)
  (`ActorComponent.SetActive` (`self.P_BeePollenA`) (`self.pollenACollected`) false)
  (`ActorComponent.SetActive` (`self.P_BeePollenB`) (`self.pollenBCollected`) false)
  (`ActorComponent.SetActive` (`self.P_BeePollenC`) (`self.pollenCCollected`) false))

(event `self.ReceiveTick`
  (params (DeltaSeconds :type "Float (single-precision)")))

(event `InputAction|Takeoff`
  (params (Key :type "Key Structure"))
  ;[1 1 1] Takeoff
  (:`Pressed`
    (bind _asabp_bee (cast `/Game/Blueprints/ABP_Bee` (`SkeletalMeshComponent.GetAnimInstance` (`self.Mesh`))))
    (set `/Game/Blueprints/ABP_Bee.InitTakeoff` true _asabp_bee)
    (`KismetSystemLibrary.Delay` (`self.TakeoffAnimLength`))
    (`self.Jump`)
    (`CharacterMovementComponent.SetMovementMode` (`self.CharacterMovement`) "MOVE_Flying" 0)
    (set `/Game/Blueprints/ABP_Bee.InitTakeoff` false _asabp_bee)))

(event `InputAxis|MoveForward`
  (params (AxisValue :type "Float (single-precision)"))
  (bind _asabp_bee (cast `/Game/Blueprints/ABP_Bee` (`SkeletalMeshComponent.GetAnimInstance` (`self.Mesh`))))
  (`/Engine/EditorBlueprintResources/StandardMacros.CompareFloat` AxisValue
    (:`>`
      (`self.AddMovementInput` (`self.GetActorForwardVector`) (* AxisValue (`self.BoostMultiplier`))))
    (:`==`)
    (:`<`
      (if (stale `self.ReceiveHit` _output_get)
        (set `/Game/Blueprints/ABP_Bee.InitLanding` true _asabp_bee)
        (`KismetSystemLibrary.Delay` (`self.LandingAnimLength`))
        (`CharacterMovementComponent.SetMovementMode` (`self.CharacterMovement`) "MOVE_None" 0)
        (set `/Game/Blueprints/ABP_Bee.InitLanding` false _asabp_bee)
        (else
          (`self.AddMovementInput` (`self.GetActorForwardVector`) (/ AxisValue (`self.ReverseSpeedDivider`))))))))

(event `InputAxis|CameraTurn`
  (params (AxisValue :type "Float (single-precision)"))
  (bind _output_get (set `self.CameraCurrentTurn` (`KismetMathLibrary.FInterpTo` (`self.CameraCurrentTurn`) (* AxisValue (`self.CameraTurnRate`)) (`GameplayStatics.GetWorldDeltaSeconds`) 1.0)))
  (`SceneComponent.K2_AddRelativeRotation` (`self.SpringArm`) (`KismetMathLibrary.MakeRotator` 0.0 0.0 _output_get) false false))

(event `self.ReceiveHit`
  (params (MyComp :type "PrimitiveComponent Object Reference") (Other :type "Actor Object Reference") (OtherComp :type "PrimitiveComponent Object Reference") (bSelfMoved :type Boolean) (HitLocation :type "Vector Structure") (HitNormal :type "Vector Structure") (NormalImpulse :type "Vector Structure") (Hit :type "HitResult Structure (by ref)"))
  (if (== (`GameplayStatics.GetObjectClass` Other) "/Script/Landscape.Landscape")
    (bind _output_get (set `self.CanLand` true))))

(event `InputAction|Boost`
  (params (Key :type "Key Structure"))
  (bind _charactermovement (`self.CharacterMovement`))
  (:`Pressed`
    (set `CharacterMovementComponent.MaxFlySpeed` (`self.BoostSpeed`) _charactermovement)
    (bind _asabp_bee (cast `/Game/Blueprints/ABP_Bee` (`SkeletalMeshComponent.GetAnimInstance` (`self.Mesh`))))
    (set `/Game/Blueprints/ABP_Bee.BoostTrue` true _asabp_bee))
  (:`Released`
    (set `CharacterMovementComponent.MaxFlySpeed` (`self.Max Fly Speed`) _charactermovement)
    (set `/Game/Blueprints/ABP_Bee.BoostTrue` false _asabp_bee)))

(event `InputAxis|CameraPitch`
  (params (AxisValue :type "Float (single-precision)"))
  (bind _springarm (`self.SpringArm`))
  (bind (_relativerotation_roll _relativerotation_pitch) (`KismetMathLibrary.BreakRotator` (`SceneComponent.RelativeRotation` _springarm)))
  (bind _output_get (set `self.CameraCurrentPitch` (`KismetMathLibrary.FInterpTo` (`self.CameraCurrentPitch`) (* AxisValue (`self.CameraTurnRate`)) (`GameplayStatics.GetWorldDeltaSeconds`) 1.0)))
  (if (`KismetMathLibrary.InRange_FloatFloat` (+ _output_get _relativerotation_pitch) -45.0 45.0)
    (`SceneComponent.K2_AddRelativeRotation` _springarm (`KismetMathLibrary.MakeRotator` 0.0 _output_get) false false)))

(fn `ReturnCamera`
  (params (TargetCam :type "Actor Object Reference"))
  (`PlayerController.SetViewTargetWithBlend` (`GameplayStatics.GetPlayerController` 0) TargetCam 2.0 "VTBlend_Linear" 0.0 false))

(fn `UserConstructionScript`)