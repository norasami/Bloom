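; BP_Wind is a wind zone actor intended to push the player bee along the wind's up vector.
; Windstream box overlaps with the bee toggle a flag and fade wind audio; Tick then offsets the bee, obtained by casting the actor's owner, by WindSpeed without delta-time scaling.
; The construction script sizes the box and counter-scales the arrow.
; Line-trace physics forces and camera-zoom timelines remain as disconnected code.
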(event `self.ReceiveTick`
  (params (DeltaSeconds :type "Float (single-precision)"))
  ;[0 1 0 1 900] Active Code
  ;;[1 1 1] Check windstream is not null
  (if (`self.BeeInWind`)
    (bind _ascbp_bee (cast `/Game/Blueprints/CBP_Bee` (`self.GetOwner`)))
    (`self.K2_AddActorWorldOffset` _ascbp_bee (* (`KismetMathLibrary.GetUpVector` (`self.K2_GetActorRotation`)) (`self.WindSpeed`)) false false)))

(event `self.Windstream.OnComponentBeginOverlap`
  (params (OverlappedComponent :type "PrimitiveComponent Object Reference") (OtherActor :type "Actor Object Reference") (OtherComp :type "PrimitiveComponent Object Reference") (OtherBodyIndex :type Integer) (bFromSweep :type Boolean) (SweepResult :type "HitResult Structure (by ref)"))
  (if (== OtherActor (`self.CBP_Bee`))
    (set `self.BeeInWind` true)
    (`KismetSystemLibrary.PrintString` "bee in wind")
    (bind _returnvalue (`AddComponent|NODE_AddAudioComponent-0`))
    (`AudioComponent.FadeIn` _returnvalue 1.0 1.0 0.0 "Linear")))

(event `self.Windstream.OnComponentEndOverlap`
  (params (OverlappedComponent :type "PrimitiveComponent Object Reference") (OtherActor :type "Actor Object Reference") (OtherComp :type "PrimitiveComponent Object Reference") (OtherBodyIndex :type Integer))
  (if (== (`self.CBP_Bee`) OtherActor)
    (set `self.BeeInWind` false)
    (`KismetSystemLibrary.PrintString` "no bee!")
    (`AudioComponent.FadeOut` (stale `self.Windstream.OnComponentBeginOverlap` _returnvalue) 1.0 0.0 "Linear")))

(fn `UserConstructionScript`
  (bind _windstream (`self.Windstream`))
  (bind (_boxextent_x _boxextent_y _boxextent_z) (`KismetMathLibrary.BreakVector` (`BoxComponent.BoxExtent` _windstream)))
  ;[0 1 0 1 225] Active Code
  ;;[1 1 1] Set dimensions and location of Windstream
  (`BoxComponent.SetBoxExtent` _windstream (`KismetMathLibrary.MakeVector` (/ (`self.WindstreamX`) 2.0) (/ (`self.WindstreamY`) 2.0) (/ (`self.WindstreamZ`) 2.0)) true)
  (`SceneComponent.K2_SetRelativeLocation` _windstream (`KismetMathLibrary.MakeVector` 0.0 0.0 _boxextent_z) false false)
  ;;[1 1 1] Keep directional arrow scale uniform
  (`SceneComponent.SetRelativeScale3D` (`self.Arrow`) (/ (1.0 1.0 1.0) (`self.GetActorScale3D`))))