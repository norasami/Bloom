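; GameManager Blueprint that decides when a flower-blooming level is won and shows the level complete screen.
; Its CheckBloomedFlowers event tests the all-bloomed flags on three referenced triggers, A, B and C, and has no caller within this graph.
; When all three are true, it creates WBP_LevelComplete, adds it to the viewport and switches the first player controller to UI-only input focused on that widget.
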(event `CheckBloomedFlowers`
  (bind _returnvalue (`GameplayStatics.GetPlayerController` 0))
  (if (and (`/Game/Blueprints/BP_TB_PollenA_Trigger.BloomedAllA` (`self.Trigger A`)) (`/Game/Blueprints/BP_TB_PollenB_Trigger.BloomedAllB` (`self.Trigger B`)) (`/Game/Blueprints/BP_TB_PollenC_Trigger.BloomedAllC` (`self.Trigger C`)))
    (bind _returnvalue_2 (`|CreateWidget` "/Game/Blueprints/WBP_LevelComplete.WBP_LevelComplete_C" _returnvalue))
    (`UserWidget.AddToViewport` _returnvalue_2 0)
    (`WidgetBlueprintLibrary.SetInputMode_UIOnlyEx` _returnvalue _returnvalue_2)))

(fn `UserConstructionScript`)