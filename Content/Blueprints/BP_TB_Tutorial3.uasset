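; BP_TB_Tutorial3 is a tutorial trigger that shows the third tutorial prompt when the bee character overlaps it.
; A DoOnce gate lets only the first overlap through, then checks the actor against the first CBP_Bee found in the level.
; On a match, it plays the Tutorial3 and TutIcon1 animations on the first WBP_TutorialAnim widget.
; The gate precedes the check, so another actor overlapping first uses up the trigger.
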(event `self.ReceiveActorBeginOverlap`
  (params (OtherActor :type "Actor Object Reference"))
  (`/Engine/EditorBlueprintResources/StandardMacros.DoOnce` false
    (:`Completed`
      (bind _outactors (`GameplayStatics.GetAllActorsOfClass` "/Game/Blueprints/CBP_Bee.CBP_Bee_C"))
      (if (== (`|GetArrayItem` _outactors) OtherActor)
        (bind _foundwidgets (`WidgetBlueprintLibrary.GetAllWidgetsOfClass` "/Game/Blueprints/WBP_TutorialAnim.WBP_TutorialAnim_C"))
        (bind _output (`|GetArrayItem` _foundwidgets))
        (`UserWidget.PlayAnimation` _output (`/Game/Blueprints/WBP_TutorialAnim.Tutorial3` _output) 0.0 1 "Forward" 1.0 false)
        (`UserWidget.PlayAnimation` _output (`/Game/Blueprints/WBP_TutorialAnim.TutIcon1` _output) 0.0 1 "Forward" 1.0 false)))))

(fn `UserConstructionScript`)