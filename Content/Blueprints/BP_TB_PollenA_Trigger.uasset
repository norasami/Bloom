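; Trigger where the player bee delivers collected pollen A, setting off the bloom of every type A flower.
; On overlap it drops the payload, blends to a cinematic camera, plays a level sequence and disables input.
; A local delayed for-each macro staggers blooms over the shuffled flowers, switching off pollen on those already bloomed.
; It then teleports the bee to a hard-coded spot, restores control and updates the GameManager's bloom progress.
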(event `self.CollisionComponent.OnComponentBeginOverlap`
  (params (OverlappedComponent :type "PrimitiveComponent Object Reference") (OtherActor :type "Actor Object Reference") (OtherComp :type "PrimitiveComponent Object Reference") (OtherBodyIndex :type Integer) (bFromSweep :type Boolean) (SweepResult :type "HitResult Structure (by ref)"))
  (bind _returnvalue (`GameplayStatics.GetPlayerPawn` 0))
  (bind _returnvalue_2 (`GameplayStatics.GetPlayerController` 0))
  (bind _or_bee (`self.OR_Bee`))
  (bind _gamemanager (`self.GameManager`))
  (bind _bee (`/Game/Blueprints/BP_Bee.Bee` (cast `/Game/Blueprints/BP_Bee` _returnvalue :!pure true)))
  ;[1 1 1] If pollen a is collected, payload drop it
  (if (== _or_bee OtherActor)
    (bind _asbp_bee (cast `/Game/Blueprints/BP_Bee` _or_bee))
    (if (`/Game/Blueprints/BP_Bee.pollenACollected` _asbp_bee)
      (`ActorComponent.Activate` (`/Game/Blueprints/BP_Bee.P_Payload_A` _asbp_bee) true)
      (set `/Game/Blueprints/BP_Bee.pollenACollected` false _asbp_bee)
      (`ActorComponent.Deactivate` (`/Game/Blueprints/BP_Bee.P_BeePollenA` _asbp_bee))
      (set `self.Player Camera` (`Controller.GetViewTarget` _returnvalue_2))
      (`PlayerController.SetViewTargetWithBlend` _returnvalue_2 (`self.Camera`) 1.0 "VTBlend_Linear" 0.0 false)
      (`MovieSceneSequencePlayer.Play` (`LevelSequenceActor.SequencePlayer` (`self.LS_Bloom_A_2`)))
      (`self.DisableInput` (`GameplayStatics.GetPlayerPawn` 0) (`GameplayStatics.GetPlayerController` 0))
      ;[1 1 1] Bloom all flowers type A that haven't bloomed
      (bind _outactors (`GameplayStatics.GetAllActorsOfClass` "/Game/Blueprints/BP_Flower_A.BP_Flower_A_C"))
      (`KismetArrayLibrary.Array_Shuffle` _outactors)
      (bind _array_element (`self.ForEachWithDelay` _outactors 0.1)
        (:`LoopBody`
          (if (`/Game/Blueprints/BP_Flower_A.hasBloomed` _array_element)
            (`/Game/Blueprints/BP_Flower_A.FlowerAPollenOff` _array_element)
            (else
              (set `/Game/Blueprints/BP_Flower_A.hasBloomed` true _array_element)
              (`SkeletalMeshComponent.Play` (`/Game/Blueprints/BP_Flower_A.aster_animation_test04` _array_element) false))))
        (:`Completed`
          ;[1 1 1] Teleport the player
          (`KismetSystemLibrary.Delay` 4.6)
          (`self.K2_TeleportTo` _returnvalue (53281.765625 -14515.654297 4433.939453) (struct :`Yaw` -90.0))
          (`PrimitiveComponent.SetPhysicsLinearVelocity` _bee (0.0 0.0 0.0) false "None")
          (`PrimitiveComponent.SetAllPhysicsAngularVelocityInDegrees` _bee (0.0 0.0 0.0) false)
          ;[1 1 1] Return camera to player
          (`PlayerController.SetViewTargetWithBlend` (`GameplayStatics.GetPlayerController` 0) (`self.Player Camera`) 1.0 "VTBlend_Linear" 0.0 false)
          (`self.EnableInput` (`GameplayStatics.GetPlayerPawn` 0) (`GameplayStatics.GetPlayerController` 0))
          ;[1 1 1] Update Game Manager
          (`KismetSystemLibrary.Delay` 1.0)
          (set `self.BloomedAllA` true)
          (`/Game/Blueprints/BP_GameManager.CheckBloomedFlowers` _gamemanager)
          (bind _result (`/Engine/EditorBlueprintResources/StandardMacros.IncrementInt` (`/Game/Blueprints/BP_GameManager.BloomedFlowers` _gamemanager))
            (:`  `
              (set `/Game/Blueprints/BP_GameManager.BloomedFlowers` _result _gamemanager))))))
    (else
      (`KismetSystemLibrary.PrintString` "Error Object Reference"))))

(fn `UserConstructionScript`)