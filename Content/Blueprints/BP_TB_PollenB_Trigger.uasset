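; Trigger that completes the Pollen B drop-off when the bee overlaps it carrying collected pollen, releasing the payload and clearing the tutorial widget.
; It blends to a cinematic camera, plays a bloom sequence with input disabled, then blooms shuffled type B flowers in a staggered delayed-loop macro.
; Afterwards it teleports the player, restores camera and input, and updates the Game Manager's bloomed-flower progress.
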(event `self.CollisionComponent.OnComponentBeginOverlap`
  (params (OverlappedComponent :type "PrimitiveComponent Object Reference") (OtherActor :type "Actor Object Reference") (OtherComp :type "PrimitiveComponent Object Reference") (OtherBodyIndex :type Integer) (bFromSweep :type Boolean) (SweepResult :type "HitResult Structure (by ref)"))
  (bind _returnvalue (`GameplayStatics.GetPlayerPawn` 0))
  (bind _or_bee (`self.OR_Bee`))
  (bind _gamemanager (`self.GameManager`))
  (bind _bee (`/Game/Blueprints/BP_Bee.Bee` (cast `/Game/Blueprints/BP_Bee` _returnvalue :!pure true)))
  ;[1 1 1] If pollen a is collected, payload drop it
  (if (== _or_bee OtherActor)
    (bind _asbp_bee (cast `/Game/Blueprints/BP_Bee` _or_bee))
    (if (`/Game/Blueprints/BP_Bee.pollenBCollected` _asbp_bee)
      (`ActorComponent.Activate` (`/Game/Blueprints/BP_Bee.P_Payload_B` _asbp_bee) true)
      (set `/Game/Blueprints/BP_Bee.pollenBCollected` false _asbp_bee)
      (`ActorComponent.Deactivate` (`/Game/Blueprints/BP_Bee.P_BeePollenB` _asbp_bee))
      ;[1 1 1] Remove tutorial
      (bind _foundwidgets (`WidgetBlueprintLibrary.GetAllWidgetsOfClass` "/Game/Blueprints/WBP_Tutorial.WBP_Tutorial_C"))
      (`Widget.RemoveFromParent` (`|GetArrayItem` _foundwidgets))
      ;[1 1 1] Blend camera to cinematic
      (`PlayerController.SetViewTargetWithBlend` (`GameplayStatics.GetPlayerController` 0) (`self.Camera`) 3.0 "VTBlend_Linear" 0.0 false)
      (`KismetSystemLibrary.Delay` 2.5)
      (`MovieSceneSequencePlayer.Play` (`LevelSequenceActor.SequencePlayer` (`self.LS_Bloom_B`)))
      (`self.DisableInput` (`GameplayStatics.GetPlayerPawn` 0) (`GameplayStatics.GetPlayerController` 0))
      ;[1 1 1] Bloom all flowers type A that haven't bloomed
      (bind _outactors (`GameplayStatics.GetAllActorsOfClass` "/Game/Blueprints/BP_Flower_B.BP_Flower_B_C"))
      (`KismetArrayLibrary.Array_Shuffle` _outactors)
      (bind _array_element (`self.ForEachWithDelay` _outactors 0.04)
        (:`LoopBody`
          (if (`/Game/Blueprints/BP_Flower_B.hasBloomed` _array_element)
            (`/Game/Blueprints/BP_Flower_B.FlowerBPollenOff` _array_element)
            (else
              (set `/Game/Blueprints/BP_Flower_B.hasBloomed` true _array_element)
              (`SkeletalMeshComponent.Play` (`/Game/Blueprints/BP_Flower_B.crocus_animation` _array_element) false))))
        (:`Completed`
          ;[1 1 1] Teleport the player
          (`KismetSystemLibrary.Delay` 0.0)
          (`self.K2_TeleportTo` _returnvalue (125.0 -21265.0 7400.0) (struct :`Yaw` 180.0))
          (`PrimitiveComponent.SetPhysicsLinearVelocity` _bee (0.0 0.0 0.0) false "None")
          (`PrimitiveComponent.SetAllPhysicsAngularVelocityInDegrees` _bee (0.0 0.0 0.0) false)
          ;[1 1 1] Return camera to player
          (`/Game/Blueprints/BP_Bee.ReturnCamera` (`self.BP_Bee`))
          (`self.EnableInput` (`GameplayStatics.GetPlayerPawn` 0) (`GameplayStatics.GetPlayerController` 0))
          ;[1 1 1] Update Game Manager
          (`KismetSystemLibrary.Delay` 1.0)
          (set `self.BloomedAllB` true)
          (`/Game/Blueprints/BP_GameManager.CheckBloomedFlowers` _gamemanager)
          (bind _result (`/Engine/EditorBlueprintResources/StandardMacros.IncrementInt` (`/Game/Blueprints/BP_GameManager.BloomedFlowers` _gamemanager))
            (:`  `
              (set `/Game/Blueprints/BP_GameManager.BloomedFlowers` _result _gamemanager))))))
    (else
      (`KismetSystemLibrary.PrintString` "Error Object Reference"))))

(fn `UserConstructionScript`)