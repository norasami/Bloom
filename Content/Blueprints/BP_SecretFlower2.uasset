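; BP_SecretFlower2 is a collectible secret flower that the bee unlocks by touching it.
; When BPBee overlaps its Box, it pauses the game, sets the GameManager's SecretFlower2Unlocked flag and updates the secret flower array.
; It then shows WBP_SecretFlower_2 on the viewport with UI-only input and destroys itself.
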(event `self.Box.OnComponentBeginOverlap`
  (params (OverlappedComponent :type "PrimitiveComponent Object Reference") (OtherActor :type "Actor Object Reference") (OtherComp :type "PrimitiveComponent Object Reference") (OtherBodyIndex :type Integer) (bFromSweep :type Boolean) (SweepResult :type "HitResult Structure (by ref)"))
  (bind _returnvalue (`GameplayStatics.GetPlayerController` 0))
  (bind _gamemanager (`self.GameManager`))
  (if (== OtherActor (`self.BP_Bee`))
    (`GameplayStatics.SetGamePaused` true)
    (set `/Game/Blueprints/BP_GameManager.SecretFlower2Unlocked` true _gamemanager)
    (`/Game/Blueprints/BP_GameManager.UpdateSecretFlowerArray` _gamemanager)
    (bind _returnvalue_2 (`|CreateWidget` "/Game/Blueprints/WBP_SecretFlower_2.WBP_SecretFlower_2_C" _returnvalue))
    (`UserWidget.AddToViewport` _returnvalue_2 0)
    (`WidgetBlueprintLibrary.SetInputMode_UIOnlyEx` _returnvalue _returnvalue_2)
    (`self.K2_DestroyActor`)))

(fn `UserConstructionScript`)